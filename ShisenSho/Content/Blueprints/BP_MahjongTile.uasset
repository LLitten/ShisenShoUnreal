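; BP_MahjongTile is a clickable mahjong tile actor that shows a face picture looked up by its TileID.
; On BeginPlay it finds BP_MahjongBoard and creates a dynamic MM_Highlight material on its cube, setting the Picture texture from DT_MahjongTile.
; Clicks are forwarded to the board, while Highlight and Unhighlight switch BaseColor between yellow and white.
; UpdateTileVisual assigns a new ID and refreshes the texture.
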(event OnClicked(Cube)
  (params (TouchedComponent :type Primitive%20Component%20Object%20Reference) (ButtonPressed :type Key%20Structure :default "None"))
  (Default|OnTileClicked (Variables|Default|GetBoard) self))

(event Custom|Unhighlight
  (Rendering|Material|SetVectorParameterValue (Variables|Default|GetDynamicMaterial) "BaseColor" "(R=1.000000,G=1.000000,B=1.000000,A=1.000000)" :!class /Script/Engine.MaterialInstanceDynamic))

(event Custom|Highlight
  (Rendering|Material|SetVectorParameterValue (Variables|Default|GetDynamicMaterial) "BaseColor" "(R=0.997412,G=1.000000,B=0.000000,A=1.000000)" :!class /Script/Engine.MaterialInstanceDynamic))

(event EventBeginPlay
  (bind _returnvalue (Actor|GetActorOfClass "/Game/Blueprints/BP_MahjongBoard.BP_MahjongBoard_C"))
  (Variables|Default|SetBoard _returnvalue)
  (bind _returnvalue_2 (Rendering|Material|CreateDynamicMaterialInstance (Variables|Default|GetCube) 0 "/Game/Materials/MM_Highlight.MM_Highlight" "" :!class /Script/Engine.PrimitiveComponent))
  (Variables|Default|SetDynamicMaterial _returnvalue_2)
  (bind _returnvalue_3 (Utilities|GetDataTableRow "/Game/DT_MahjongTile.DT_MahjongTile" (Utilities|String|StringToName (Utilities|String|ToString(Integer) (Variables|Default|GetTileID))))
    (:then
      (Rendering|Material|SetTextureParameterValue (Variables|Default|GetDynamicMaterial) "Picture" (Utilities|Struct|BreakS_MahjongTileData _returnvalue_3)))))

(event Collision|EventActorBeginOverlap
  (params (OtherActor :type Actor%20Object%20Reference)))

(event EventTick
  (params (DeltaSeconds :type Float%20%28single-precision%29)))

(fn ConstructionScript)

(fn UpdateTileVisual
  (params (NewID :type Integer))
  (Variables|Default|SetTileID NewID)
  (bind _returnvalue (Utilities|GetDataTableRow "/Game/DT_MahjongTile.DT_MahjongTile" (Utilities|String|StringToName (Utilities|String|ToString(Integer) (Variables|Default|GetTileID))))
    (:then
      (Rendering|Material|SetTextureParameterValue (Variables|Default|GetDynamicMaterial) "Picture" (Utilities|Struct|BreakS_MahjongTileData _returnvalue)))))