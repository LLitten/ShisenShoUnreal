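; Game mode for a Mahjong tile game that sets up the view, cursor and HUD and runs the match timer.
; On BeginPlay it switches to the scene's camera, creates WBP_HUD, then counts BP_MahjongBoard's active tiles after short delays that let spawning finish.
; A one-second looping timer advances combo and elapsed time, updates the HUD clock, and at zero tiles computes a time-decaying bonus and shows WBP_EndScreen.
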(event Custom|TimerTick
  ;[0.15 0.15 0.15 0.5] Gameplay Timer
  ;;[0.15 0.15 0.15 0.5] Combo timer
  (Variables|Default|SetComboTimer (+ (Variables|Default|GetComboTimer) 1))
  (bind _output_get (Variables|Default|SetTimeElapsed (+ (Variables|Default|GetTimeElapsed) 1)))
  (Default|UpdateTimerUI (Variables|Default|GetHUD_Reference) (Utilities|Text|ToText(String) (Utilities|String|Left (Class|KismetStringLibrary|TimeSecondstoString (Math|Conversions|ToFloat(Integer) _output_get)) 5)))
  ;;[0.15 0.15 0.15 0.5] Stop timer when there are no tiles left
  (if (== (Variables|Default|GetTilesRemaining) 0)
    (Utilities|Time|ClearandInvalidateTimerbyHandle (stale EventBeginPlay _returnvalue_5))
    ;[0.15 0.15 0.15 0.5] Bonus score for completing the game fast
    (Variables|Default|SetTimeBonus (Math|Integer|Max(Integer) (- 5000 (* (Variables|Default|GetTimeElapsed) 50))))
    ;[0.15 0.15 0.15 0.5] Make end screen
    (bind _returnvalue (UserInterface|CreateWidget "/Game/Blueprints/WBP_EndScreen.WBP_EndScreen_C"))
    (bind _output_get_2 (Variables|Default|SetEndScreen_Reference _returnvalue))
    (UserInterface|Viewport|AddtoViewport _output_get_2 0)))

(event EventBeginPlay
  (bind _returnvalue (Game|GetPlayerController 0))
  (Utilities|FlowControl|Delay 0.2) ; idk it helps editor not freak out
  ;[0.15 0.15 0.15 0.5] Set view to be at above camera
  (bind _returnvalue_2 (Actor|GetActorOfClass "/Script/Engine.CameraActor"))
  (Game|Player|SetViewTargetwithBlend _returnvalue _returnvalue_2 0.0 "VTBlend_Linear" 0.0 false)
  ;[0.15 0.15 0.15 0.5] Stop cursor from being restricted to UI
  (Input|SetInputModeGameandUI _returnvalue 0 "DoNotLock" false false)
  (Variables|/Script/Engine.PlayerController|SetbShowMouseCursor _returnvalue true)
  (Class|WidgetBlueprintLibrary|SetFocustoGameViewport)
  ;[0.15 0.15 0.15 0.5] Create HUD
  (bind _returnvalue_3 (UserInterface|CreateWidget "/Game/Blueprints/WBP_HUD.WBP_HUD_C"))
  (bind _output_get (Variables|Default|SetHUD_Reference _returnvalue_3))
  (UserInterface|Viewport|AddtoViewport _output_get 0)
  (bind _returnvalue_4 (Actor|GetActorOfClass "/Game/Blueprints/BP_MahjongBoard.BP_MahjongBoard_C"))
  ;[0.15 0.15 0.15 0.5] Count number of tiles spawned
  (Utilities|FlowControl|Delay 0.2) ; Make sure Unreal doesn't go too fast and count the tiles before they're done spawning
  (bind _output_get_2 (Variables|Default|SetTilesRemaining (Utilities|Map|Length (Variables|/Game/Blueprints/BP_MahjongBoard.BP_MahjongBoard_C|GetActiveTiles _returnvalue_4))))
  (Default|UpdateTileCountUI (Variables|Default|GetHUD_Reference) _output_get_2)
  ;[0.15 0.15 0.15 0.5] Gameplay Timer
  (bind _returnvalue_5 (Utilities|Time|SetTimerbyEvent (delegate Custom|TimerTick) 1.0 true)))

(event EventTick
  (params (DeltaSeconds :type Float%20%28single-precision%29)))

(fn ConstructionScript)